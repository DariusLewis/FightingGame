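; Radio Blueprint that plays continuous background music by picking random tracks from SongList, starting on BeginPlay.
; ChangeSong fades out any still-valid track, spawns the next as a 2D sound, then re-calls itself after a delay equal to that song's duration.
; Selection is purely random, so tracks can repeat back to back.
; It is set tickable when paused, and StopMusic fades the current track and blocks further changes.
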(event Custom|Change%20Song
  ;[1 1 1] Change Song
  (if (Variables|Default|GetCan%20Play%20Song)
    (bind _isfading (CallFunction|TryFadeOut))
    (if _isfading
      (Utilities|FlowControl|Delay (Variables|Default|GetFade%20Out%20Duration)))
    (bind _output_get (Variables|Default|SetCurrentSong (CallFunction|SelectNewSong)))
    (bind _returnvalue (Audio|SpawnSound2D _output_get (Variables|Default|GetVolune) 1.0 0.0 0))
    (Variables|Default|SetCurrentSongRef _returnvalue)
    (Utilities|FlowControl|Delay (Variables|/Script/Engine.SoundBase|GetDuration _output_get))
    (CallFunction|ChangeSong)))

(event Custom|StopMusic
  ;[1 1 1] Stop Music
  (Audio|Components|Audio|FadeOut (Variables|Default|GetCurrentSongRef) 1.0 0.0 "Linear" :!class /Script/Engine.AudioComponent)
  (Variables|Default|SetCan%20Play%20Song false))

(event EventBeginPlay
  ;[1 1 1] Start Music
  (Variables|Default|SetCan%20Play%20Song true)
  (Class|Actor|SetTickablewhenPaused true)
  (CallFunction|ChangeSong))

(fn ConstructionScript)

(fn SelectNewSong
  (bind _songlist (Variables|Default|GetSongList))
  (bind _output_get (Variables|Default|SetProvisinal%20Song (Utilities|Array|Get(acopy) _songlist (Math|Random|RandomIntegerinRange 0 (Utilities|Array|LastIndex _songlist)))))
  (return _output_get))

(fn TryFadeOut
  (bind _currentsongref (Variables|Default|GetCurrentSongRef)
    (:then
      (Audio|Components|Audio|FadeOut _currentsongref (Variables|Default|GetFade%20Out%20Duration) 0.0 "Linear" :!class /Script/Engine.AudioComponent)
      (return true))
    (:else
      (return false))))